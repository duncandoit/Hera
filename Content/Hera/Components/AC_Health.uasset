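; Health component that tracks a layered pool of health, shields, armor, overshield and overarmor, destroying its owner when health reaches zero.
; On BeginPlay it loads DA_TestHealth, filling health, shields and armor to their maximums while keeping existing over-values.
; Damage drains overarmor, overshield, armor, shields, then health, using a clamped subtraction helper to carry leftover damage into the next layer.
; SetHealthPool stores the result and performs the death check.
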(event `self.ReceiveBeginPlay`
  (`self.SetHealthData` "/Game/Hera/Data/DA_TestHealth.DA_TestHealth"))

(fn `Damage`
  (params (NewDamage :type Integer))
  (locals (LHealth :type Integer) (LShields :type Integer) (LArmor :type Integer) (LOverShields :type Integer) (LOverArmor :type Integer))
  (bind (_healthpool_health _healthpool_shields _healthpool_armor _healthpool_overshield _healthpool_overarmor) (break `/Game/Hera/STRUCT_Health` (`self.HealthPool`)))
  (bind _output_get (set `local.LOverArmor` _healthpool_overarmor))
  (bind _output_get_2 (set `local.LOverShields` _healthpool_overshield))
  (bind _output_get_3 (set `local.LArmor` _healthpool_armor))
  (bind _output_get_4 (set `local.LShields` _healthpool_shields))
  (bind _output_get_5 (set `local.LHealth` _healthpool_health))
  (bind (_valueiszeroorless _normalizednewhealthvalue _remainingsubtractionamount) (`self.NormalizedHealthValueSubtracted` _output_get NewDamage))
  (set `local.LOverArmor` _normalizednewhealthvalue)
  (if _valueiszeroorless
    (bind (_valueiszeroorless_2 _normalizednewhealthvalue_2 _remainingsubtractionamount_2) (`self.NormalizedHealthValueSubtracted` _output_get_2 _remainingsubtractionamount))
    (set `local.LOverShields` _normalizednewhealthvalue_2)
    (if _valueiszeroorless_2
      (bind (_valueiszeroorless_3 _normalizednewhealthvalue_3 _remainingsubtractionamount_3) (`self.NormalizedHealthValueSubtracted` _output_get_3 _remainingsubtractionamount_2))
      (set `local.LArmor` _normalizednewhealthvalue_3)
      (if _valueiszeroorless_3
        (bind (_valueiszeroorless_4 _normalizednewhealthvalue_4 _remainingsubtractionamount_4) (`self.NormalizedHealthValueSubtracted` _output_get_4 _remainingsubtractionamount_3))
        (set `local.LShields` _normalizednewhealthvalue_4)
        (if _valueiszeroorless_4
          (bind (_valueiszeroorless_5 _normalizednewhealthvalue_5) (`self.NormalizedHealthValueSubtracted` _output_get_5 _remainingsubtractionamount_4))
          (set `local.LHealth` _normalizednewhealthvalue_5)))))
  (`self.SetHealthPool` (make `/Game/Hera/STRUCT_Health` (`local.LHealth`) (`local.LShields`) (`local.LArmor`) (`local.LOverShields`) (`local.LOverArmor`)))
  (return))

(fn `GetHealthData`
  (returns (Data :type "LifePoolData Object Reference"))
  (return (`self.HealthData`)))

(fn `GetHealthPool`
  (returns (NewParam :type "/Game/Hera/STRUCT_Health Structure"))
  (return (`self.HealthPool`)))

(fn `NormalizedHealthValueSubtracted`
  (params (StartingHealthValue :type Integer) (SubtractedAmount :type Integer))
  (returns (ValueIsZeroOrLess :type Boolean) (NormalizedNewHealthValue :type Integer) (RemainingSubtractionAmount :type Integer))
  (bind _returnvalue (- StartingHealthValue SubtractedAmount))
  (if (<= _returnvalue 0)
    (return true 0 (* _returnvalue -1))
    (else
      (return false _returnvalue 0))))

(fn `SetHealthData`
  (params (NewData :type "LifePoolData Object Reference"))
  (bind (_healthpool_health _healthpool_shields _healthpool_armor _healthpool_overshield _healthpool_overarmor) (break `/Game/Hera/STRUCT_Health` (`self.HealthPool`)))
  (bind _output_get (set `self.HealthData` NewData))
  (set `self.HealthPool` (make `/Game/Hera/STRUCT_Health` (`LifePoolData.MaxHealth` _output_get) (`LifePoolData.MaxShields` _output_get) (`LifePoolData.MaxArmor` _output_get) _healthpool_overshield _healthpool_overarmor)))

(fn `SetHealthPool`
  (params (NewHealth :type "/Game/Hera/STRUCT_Health Structure"))
  (bind _healthpool_health (break `/Game/Hera/STRUCT_Health` (`self.HealthPool`)))
  (set `self.HealthPool` NewHealth)
  (if (<= _healthpool_health 0)
    (`Actor.K2_DestroyActor` (`self.GetOwner`))))