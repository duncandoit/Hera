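; Gameplay ability that lets a falling character take a limited chain of mid-air steps while input is held.
; On authority, a looping delay task fires TakeStep, which zeroes movement and applies an impulse from last input direction plus a gravity- and mass-scaled lift.
; Releasing input during stepping adds a smaller closing impulse and exhausts the steps.
; Switching to Walking resets the count, clears tasks and ends the ability.
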(event `self.K2_ActivateAbility`
  (`self.StartStepping`))

(event `StartStepping`
  (bind _returnvalue (`Actor.GetComponentByClass` (`self.GetAvatarActorFromActorInfo`) "/Script/Engine.CharacterMovementComponent"))
  (bind _returnvalue_2 (/ (`self.StepLength`) 2.0))
  (bind (_newimpulsex _newimpulsey) (`self.ImpulseHorizontalStrength` _returnvalue_2))
  (`/Engine/EditorBlueprintResources/StandardMacros.IsValid` _returnvalue
    (:`Is Valid`
      (set `self.Character Movement` _returnvalue)
      (`self.K2_CommitAbility`)
      (`self.K2_HasAuthority`
        (:`True`
          (bind _asynctaskproxy (`AbilityTask_WaitMovementModeChange.CreateWaitMovementModeChange` "MOVE_Walking")
            (:`then`
              (set `self.Landing Task` _asynctaskproxy)
              (bind _asynctaskproxy_2 (`AbilityTask_WaitInputRelease.WaitInputRelease` true)
                (:`then`
                  (bind _releasetask (`self.ReleaseTask`)
                    (:`then`
                      (`GameplayTask.EndTask` _releasetask))
                    (:`else`
                      _))
                  (set `self.ReleaseTask` _asynctaskproxy_2)
                  (bind _asynctaskproxy_3 (`GameplayTask_WaitDelay.TaskWaitDelay` null (/ (`self.StepDurationMS`) 50.0) :!label _label)
                    (:`then`
                      (bind _steptask (`self.StepTask`)
                        (:`then`
                          (`GameplayTask.EndTask` _steptask))
                        (:`else`
                          _))
                      (set `self.StepTask` _asynctaskproxy_3)
                      (`self.TakeStep`))
                    (:`OnFinish`
                      (if (< (`self.StepsTaken`) (`self.MaxSteps`))
                        (goto _label)
                        (else
                          (bind _steptask_2 (`self.StepTask`)
                            (:`then`
                              (`GameplayTask.EndTask` _steptask_2)
                              (bind _releasetask_2 (`self.ReleaseTask`)
                                (:`then`
                                  (`GameplayTask.EndTask` _releasetask_2))
                                (:`else`)))
                            (:`else`)))))))
                (:`OnRelease`
                  (bind _steptask_3 (`self.StepTask`)
                    (:`then`
                      (`GameplayTask.EndTask` _steptask_3)
                      (set `self.StepsTaken` (`self.MaxSteps`))
                      (`CharacterMovementComponent.AddImpulse` (`self.Character Movement`) (`KismetMathLibrary.MakeVector` _newimpulsex _newimpulsey _returnvalue_2) false))
                    (:`else`)))))
            (:`OnChange`
              (`self.Reset`))))))
    (:`Is Not Valid`
      (`self.K2_EndAbility`))))

(event `Reset`
  (set `self.StepsTaken` 0)
  (bind _steptask (`self.StepTask`)
    (:`then`
      (`GameplayTask.EndTask` _steptask))
    (:`else`
      _))
  (bind _releasetask (`self.ReleaseTask`)
    (:`then`
      (`GameplayTask.EndTask` _releasetask))
    (:`else`
      _))
  (bind _landing_task (`self.Landing Task`)
    (:`then`
      (`GameplayTask.EndTask` _landing_task))
    (:`else`
      _))
  (`self.K2_EndAbility`))

(fn `ImpulseHorizontalStrength`
  (params (Length :type "Float (double-precision)"))
  (returns (NewImpulseX :type "Float (double-precision)") (NewImpulseY :type "Float (double-precision)"))
  (bind (_returnvalue_x _returnvalue_y) (`KismetMathLibrary.BreakVector` (`PawnMovementComponent.GetLastInputVector` (`self.Character Movement`))))
  (return (* _returnvalue_x Length) (* _returnvalue_y Length)))

(fn `ImpulseVerticalStrength`
  (params (AirTime :type "Float (double-precision)") (Height :type "Float (double-precision)"))
  (returns (NewImpulseHeight :type "Float (double-precision)"))
  (locals (ImpulseZ :type "Float (double-precision)"))
  (bind _character_movement (`self.Character Movement`))
  (bind _output_get (set `local.ImpulseZ` (* AirTime (`CharacterMovementComponent.Mass` _character_movement) (/ (`KismetMathLibrary.Abs` (`MovementComponent.GetGravityZ` _character_movement)) 100.0))))
  (return (+ _output_get Height)))

(fn `K2_CanActivateAbility`
  (params (ActorInfo :type "GameplayAbilityActorInfo Structure") (Handle :type "GameplayAbilitySpecHandle Structure"))
  (returns (RelevantTags :type "GameplayTagContainer Structure") (ReturnValue :type Boolean))
  (bind _ascharacter (cast `Character` ActorInfo_AvatarActor)
    (:`then`
      (return (struct) (and (`NavMovementComponent.IsFalling` (`Character.CharacterMovement` _ascharacter)) (< (`self.StepsTaken`) (`self.MaxSteps`)))))
    (:`CastFailed`
      (return (struct) false))))

(fn `TakeStep`
  (bind (_newimpulsex _newimpulsey) (`self.ImpulseHorizontalStrength` (`self.StepLength`)))
  (`MovementComponent.StopMovementImmediately` (`self.Character Movement`))
  (`CharacterMovementComponent.AddImpulse` (`self.Character Movement`) (`KismetMathLibrary.MakeVector` _newimpulsex _newimpulsey (`self.ImpulseVerticalStrength` (`self.StepDurationMS`) (`self.StepExtraHeight`))) false)
  (`/Engine/EditorBlueprintResources/StandardMacros.IncrementInt` (`self.StepsTaken`)))