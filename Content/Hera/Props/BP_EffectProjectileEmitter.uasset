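; BP_EffectProjectileEmitter is a prop actor that repeatedly fires effect projectiles from its own transform.
; A looping one-second timer started on BeginPlay spawns a BP_EffectProjectile, adjusting its position on collision but always spawning.
; Each new projectile receives the emitter's Effect, Level and projectile material, so the emitter's variables define what it launches.
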(event `self.ReceiveBeginPlay`
  (`KismetSystemLibrary.K2_SetTimerDelegate` (delegate `EmitProjectile`) 1.0 true))

(event `EmitProjectile`
  (bind _returnvalue (`|SpawnActorFromClass` "/Game/Hera/Props/BP_EffectProjectile.BP_EffectProjectile_C" (`self.GetTransform`) "AdjustIfPossibleButAlwaysSpawn" "OverrideRootScale" null (struct) null))
  (set `/Game/Hera/Props/BP_EffectProjectile.Effect` (`self.Effect`) _returnvalue)
  (set `/Game/Hera/Props/BP_EffectProjectile.Level` (`self.Level`) _returnvalue)
  (`PrimitiveComponent.SetMaterial` (`/Game/Hera/Props/BP_EffectProjectile.Projectile` _returnvalue) 0 (`self.ProjectileMaterial`)))

(fn `UserConstructionScript`)